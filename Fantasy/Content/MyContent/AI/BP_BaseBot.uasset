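; Base sword-fighting AI bot with a health bar widget and a damage interface routed to its damage system component.
; Drawing and sheathing play montages and set the battle state, while a flip-flop event moves the sword between battle and default sockets.
; The default attack plays a slash montage and sphere-traces forward for pawns, sending blockable damage.
; Death disables capsule collision; Heal is a stub returning zero.
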(event `self.ReceiveBeginPlay`
  (bind _returnvalue (`|CreateWidget` "/Game/MyContent/DamageSystem/HealthBar.HealthBar_C" null self))
  (`WidgetComponent.SetWidget` (`self.HealthBar`) _returnvalue))

(event `/Game/MyContent/AI/BI_BaseBot.ReplaceSword`
  (`/Engine/EditorBlueprintResources/StandardMacros.FlipFlop`
    (:`A`
      (`SceneComponent.K2_AttachToComponent` (`self.Sword`) (`self.BattleSwordSocket`) "None" "KeepRelative" "KeepRelative" "KeepRelative" true))
    (:`B`
      (`SceneComponent.K2_AttachToComponent` (`self.Sword`) (`self.DefaultSwordSocket`) "None" "KeepRelative" "KeepRelative" "KeepRelative" true))))

(event `Death`
  (`PrimitiveComponent.SetCollisionEnabled` (`self.CapsuleComponent`) "NoCollision"))

(fn `DefaultAttack`
  (returns (Delay :type "Float (double-precision)"))
  (bind _returnvalue (`self.K2_GetActorLocation`))
  (bind _returnvalue_2 (`self.PlayAnimMontage` "/Game/MyContent/Character/Animations/SwordRightSlash_Montage.SwordRightSlash_Montage"))
  (bind (_outhit _returnvalue_3) (`KismetSystemLibrary.SphereTraceSingleForObjects` :`Start` _returnvalue :`End` (+ _returnvalue (* (`self.GetActorForwardVector`) 200.0)) :`Radius` 20.0 :`ObjectTypes` (`|MakeArray` "ObjectTypeQuery3" :!type "EObjectTypeQuery Enum") :`DrawDebugType` "ForDuration" :`DrawTime` 1.0))
  (if _returnvalue_3
    (message `/Game/MyContent/DamageSystem/BPI_Damagable.TakeDamage` (`.HitActor` (`GameplayStatics.BreakHitResult` _outhit)) (make `/Game/MyContent/DamageSystem/S_DamageInfo` 20.0 "NewEnumerator1" "NewEnumerator0" true)))
  (return _returnvalue_2))

(fn `DrawSword`
  (returns (Delay :type "Float (double-precision)"))
  (bind _returnvalue (`self.PlayAnimMontage` "/Game/MyContent/Character/Animations/DrawSword_Montage.DrawSword_Montage"))
  (set `self.BattleState` true)
  (return _returnvalue))

(fn `GetCurrentHealth`
  (returns (Health :type "Float (double-precision)"))
  (return (`/Game/MyContent/DamageSystem/BPC_DamageSystem.Health` (`self.BPC_DamageSystem`))))

(fn `GetMaxHealth`
  (returns (Health :type "Float (double-precision)"))
  (return (`/Game/MyContent/DamageSystem/BPC_DamageSystem.MaxHealth` (`self.BPC_DamageSystem`))))

(fn `Heal`
  (params (Heal :type "Float (double-precision)"))
  (returns (NewHealth :type "Float (double-precision)"))
  (return 0.0))

(fn `SheathSword`
  (returns (Delay :type "Float (double-precision)"))
  (bind _returnvalue (`self.PlayAnimMontage` "/Game/MyContent/Character/Animations/SheathSword_Montage.SheathSword_Montage"))
  (set `self.BattleState` false)
  (return _returnvalue))

(fn `TakeDamage`
  (params (DamageInfo :type "/Game/MyContent/DamageSystem/S_DamageInfo Structure"))
  (returns (WasDamaged :type Boolean))
  (bind _wasdamaged (`/Game/MyContent/DamageSystem/BPC_DamageSystem.TakeDamage` (`self.BPC_DamageSystem`) DamageInfo))
  (return _wasdamaged))

(fn `UserConstructionScript`
  (add `/Game/MyContent/DamageSystem/BPC_DamageSystem.OnDeath` (`self.BPC_DamageSystem`) (`|CreateDelegate` :!event `Death`)))