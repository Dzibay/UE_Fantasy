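; BPC_DamageSystem is a damage component that tracks health, blocking and death for its owner.
; TakeDamage routes through CanBeDamaged, which allows damage only when alive and either not blocking or facing an unblockable hit.
; Damage reduces Health, sets IsDead and calls OnDeath at zero or below, and returns true.
; Any rejected hit, including one on an already dead target, calls OnBlocked and returns false.
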(event `self.ReceiveTick`
  (params (DeltaSeconds :type "Float (single-precision)")))

(fn `TakeDamage`
  (params (DamageInfo :type "/Game/MyContent/DamageSystem/S_DamageInfo Structure"))
  (returns (WasDamaged :type Boolean))
  (bind (_damage _damagetype _damageeffect _canbeblocked) (break `/Game/MyContent/DamageSystem/S_DamageInfo` DamageInfo))
  (`self.CanBeDamaged` _canbeblocked
    (:`Damage`
      (bind _output_get (set `self.Health` (- (`self.Health`) _damage)))
      (if (<= _output_get 0.0)
        (set `self.IsDead` true)
        (`self.OnDeath`))
      (return true))
    (:`Block`
      (`self.OnBlocked`)
      (return false))))