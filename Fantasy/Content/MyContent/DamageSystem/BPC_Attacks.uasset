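; Attack component in the damage system that applies damage to hit actors who are not on its owner's team.
; DamageAllNotTeamMembers loops over hit results, compares each actor's team with the owner's through message calls, and sends TakeDamage with the damage info and owner as instigator.
; It records damaged actors to avoid hitting one twice and returns that list.
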(fn `DamageAllNotTeamMembers`
  (params (Hits :type "Array of HitResult Structure") (DamageInfo :type "/Game/MyContent/DamageSystem/S_DamageInfo Structure"))
  (returns (DamagedActors :type "Array of Actor Object Reference"))
  (locals (DamagedActor :type "Array of Actor Object Reference"))
  (for _array_element Hits
    (bind (_bblockinghit _binitialoverlap _time _distance _location _impactpoint _normal _impactnormal _physmat _hitactor) (`GameplayStatics.BreakHitResult` _array_element))
    (bind _teamnumber (message `/Game/MyContent/DamageSystem/BPI_Damagable.GetTeam` _hitactor))
    (bind _teamnumber_2 (message `/Game/MyContent/DamageSystem/BPI_Damagable.GetTeam` (`self.GetOwner`)))
    (if (and (!= _teamnumber_2 _teamnumber) (not (`KismetArrayLibrary.Array_Contains` (`local.DamagedActor`) _hitactor)))
      (message `/Game/MyContent/DamageSystem/BPI_Damagable.TakeDamage` _hitactor DamageInfo (`self.GetOwner`))
      (`KismetArrayLibrary.Array_AddUnique` (`local.DamagedActor`) _hitactor)))
  (return (`local.DamagedActor`)))